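; BP_Helmet is a helmet item pickup that the player collects by walking into its sphere.
; On BeginPlay the sphere's collision is off, then switches to query-only after a short delay, so pickup is not immediate.
; An overlapping BP_TestPlayer has ItemInfo and DroppedAmount passed to its InventoryComponent's AddItem.
; The actor destroys itself only when AddItem succeeds.
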(event `self.ReceiveBeginPlay`
  (`PrimitiveComponent.SetCollisionEnabled` (`self.Sphere`) "NoCollision")
  (`KismetSystemLibrary.Delay` 2.0)
  (`PrimitiveComponent.SetCollisionEnabled` (`self.Sphere`) "QueryOnly"))

(event `self.Sphere.OnComponentBeginOverlap`
  (params (OverlappedComponent :type "PrimitiveComponent Object Reference") (OtherActor :type "Actor Object Reference") (OtherComp :type "PrimitiveComponent Object Reference") (OtherBodyIndex :type Integer) (bFromSweep :type Boolean) (SweepResult :type "HitResult Structure (by ref)"))
  (bind _asbp_test_player (cast `/Game/BP_TestPlayer` OtherActor))
  (bind _returnvalue (`InventoryComponent.AddItem` (`self.GetComponentByClass` _asbp_test_player "/Script/MarketplacePlugins.InventoryComponent") (`self.ItemInfo`) (`self.DroppedAmount`)))
  (if _returnvalue
    (`self.K2_DestroyActor`)))

(fn `UserConstructionScript`)