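; BP_IronOre is an iron ore pickup that players can collect into their inventory.
; Sphere overlap sets or clears itself as BP_TestPlayer's CurrentPickupItem and refreshes that player's pickup hint.
; Server_PickupItem adds ItemInfo and DroppedAmount to the player's InventoryComponent, then clears the reference and destroys the actor on success.
; A dynamic material on Cube supports highlight toggling, but the highlight calls in the event graph are unconnected.
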(event `self.ReceiveBeginPlay`
  (bind _returnvalue (`PrimitiveComponent.CreateDynamicMaterialInstance` (`self.Cube`) 0 null "None"))
  (set `self.HighlightMID` _returnvalue)
  (`MaterialInstanceDynamic.SetScalarParameterValue` (`self.HighlightMID`) "HighlightIntensity" 0.0))

(event `self.Sphere.OnComponentBeginOverlap`
  (params (OverlappedComponent :type "PrimitiveComponent Object Reference") (OtherActor :type "Actor Object Reference") (OtherComp :type "PrimitiveComponent Object Reference") (OtherBodyIndex :type Integer) (bFromSweep :type Boolean) (SweepResult :type "HitResult Structure (by ref)"))
  (bind _asbp_test_player (cast `/Game/BP_TestPlayer` OtherActor))
  (set `/Game/BP_TestPlayer.CurrentPickupItem` self _asbp_test_player)
  (`/Game/BP_TestPlayer.UpdatePickupHint` _asbp_test_player))

(event `self.Sphere.OnComponentEndOverlap`
  (params (OverlappedComponent :type "PrimitiveComponent Object Reference") (OtherActor :type "Actor Object Reference") (OtherComp :type "PrimitiveComponent Object Reference") (OtherBodyIndex :type Integer))
  (bind _asbp_test_player (cast `/Game/BP_TestPlayer` OtherActor))
  (if (== (`/Game/BP_TestPlayer.CurrentPickupItem` _asbp_test_player) self)
    (set `/Game/BP_TestPlayer.CurrentPickupItem` null _asbp_test_player)
    (`/Game/BP_TestPlayer.UpdatePickupHint` _asbp_test_player)))

(event `Server_PickupItem`
  (params (PlayerRef :type "/Game/BP_TestPlayer Object Reference"))
  (`/Engine/EditorBlueprintResources/StandardMacros.IsValid` PlayerRef
    (:`Is Valid`
      (bind _returnvalue (`InventoryComponent.TryAddItem` (`self.GetComponentByClass` PlayerRef "/Script/MarketplacePlugins.InventoryComponent") (`self.ItemInfo`) (`self.DroppedAmount`)))
      (if _returnvalue
        (set `/Game/BP_TestPlayer.CurrentPickupItem` null PlayerRef)
        (`self.K2_DestroyActor`)))))

(fn `DisableHighlight`
  (bind _highlightmid (`self.HighlightMID`))
  (`/Engine/EditorBlueprintResources/StandardMacros.IsValid` _highlightmid
    (:`Is Valid`
      (`MaterialInstanceDynamic.SetScalarParameterValue` _highlightmid "HighlightIntensity" 0.0)
      (`KismetSystemLibrary.PrintString` "\"DisableHighlight called\""))))

(fn `EnableHighlight`
  (bind _highlightmid (`self.HighlightMID`))
  (`/Engine/EditorBlueprintResources/StandardMacros.IsValid` _highlightmid
    (:`Is Valid`
      (`MaterialInstanceDynamic.SetScalarParameterValue` _highlightmid "HighlightIntensity" 50.0)
      (`KismetSystemLibrary.PrintString` "\"EnableHighlight called\""))))

(fn `UserConstructionScript`)